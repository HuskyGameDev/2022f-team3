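; Base enemy Blueprint with pawn sensing, a health value and logic for following the player.
; The construction script initializes Health from DefaultHealth, while the AnyDamage event is empty.
; FollowPlayer issues an AI MoveTo toward player character 0 only when SeePlayer is true.
; OnSeePawn sets SeePlayer to false before calling FollowPlayer, so sighting a pawn does not start the chase as wired.
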(event OnSeePawn(PawnSensing)
  (params (Pawn :type Pawn%20Object%20Reference))
  (Variables|Default|SetSeePlayer false)
  (CallFunction|FollowPlayer))

(event Custom|FollowPlayer
  (if (Variables|Default|GetSeePlayer)
    (AI|AIMoveTo self "0, 0, 0" (Game|GetPlayerCharacter 0) 5.0 false)))

(event Game|Damage|EventAnyDamage
  (params (Damage :type Float%20%28single-precision%29) (DamageType :type Damage%20Type%20Object%20Reference) (InstigatedBy :type Controller%20Object%20Reference) (DamageCauser :type Actor%20Object%20Reference)))

(fn ConstructionScript
  (Variables|Default|Sethealth (Variables|Default|Getdefault%20health)))